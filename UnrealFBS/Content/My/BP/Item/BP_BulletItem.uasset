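; BP_BulletItem is an ammo pickup that refills the first-person character's ammo when touched.
; Its static mesh spins on yaw every Tick at RotateSpeed.
; On overlap with BP_FirstPersonCharacter, it sets the current ammo to a fixed full amount rather than adding to it.
; The mesh then hides and disables collision, reappearing after a short delay, so the same actor respawns without being destroyed.
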(event `self.ReceiveTick`
  (params (DeltaSeconds :type "Float (single-precision)"))
  (`SceneComponent.K2_AddRelativeRotation` (`self.StaticMesh`) (`KismetMathLibrary.MakeRotator` 0.0 0.0 (* DeltaSeconds (`self.RotateSpeed`))) false false))

(event `self.StaticMesh.OnComponentBeginOverlap`
  (params (OverlappedComponent :type "PrimitiveComponent Object Reference") (OtherActor :type "Actor Object Reference") (OtherComp :type "PrimitiveComponent Object Reference") (OtherBodyIndex :type Integer) (bFromSweep :type Boolean) (SweepResult :type "HitResult Structure (by ref)"))
  (bind _staticmesh (`self.StaticMesh`))
  (bind _staticmesh_2 (`self.StaticMesh`))
  (bind _asbp_first_person_character (cast `/Game/My/BP/BP_FirstPersonCharacter` OtherActor))
  (set `/Game/My/BP/BP_FirstPersonCharacter.Player Current Ammo` 30 _asbp_first_person_character)
  (`SceneComponent.SetHiddenInGame` _staticmesh true false)
  (`PrimitiveComponent.SetCollisionEnabled` _staticmesh "NoCollision")
  (`KismetSystemLibrary.Delay` 3.0)
  (`SceneComponent.SetHiddenInGame` _staticmesh_2 false false)
  (`PrimitiveComponent.SetCollisionEnabled` _staticmesh_2 "QueryAndPhysics"))

(fn `UserConstructionScript`)