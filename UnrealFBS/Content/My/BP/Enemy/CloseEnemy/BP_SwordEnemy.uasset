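; AI controller for the sword-wielding close-combat enemy that runs the BT_EnemySword behavior tree on begin play and prints a debug string.
; AI Perception updates react only to BP_FirstPersonCharacter, writing it to the Player blackboard key and switching the AI_Status enum between sensed and lost states.
; Losing perception keeps the player reference in the blackboard, so only the status value distinguishes the two states.
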(event `self.ReceiveBeginPlay`
  (`self.RunBehaviorTree` "/Game/My/BP/Enemy/CloseEnemy/BT_EnemySword.BT_EnemySword")
  (`KismetSystemLibrary.PrintString` "12414"))

(event `self.AIPerception.OnTargetPerceptionUpdated`
  (params (Actor :type "Actor Object Reference") (Stimulus :type "AIStimulus Structure"))
  (bind _asbp_first_person_character (cast `/Game/My/BP/BP_FirstPersonCharacter` Actor))
  (if (`.bSuccessfullySensed` (break `AIStimulus` Stimulus))
    (`BlackboardComponent.SetValueAsObject` (`AIBlueprintHelperLibrary.GetBlackboard` null) "Player" _asbp_first_person_character)
    (`BlackboardComponent.SetValueAsEnum` (`AIBlueprintHelperLibrary.GetBlackboard` null) "AI_Status" (enumliteral `/Game/My/BP/Enemy/AI_Status` "NewEnumerator1"))
    (else
      (`BlackboardComponent.SetValueAsObject` (`AIBlueprintHelperLibrary.GetBlackboard` null) "Player" _asbp_first_person_character)
      (`BlackboardComponent.SetValueAsEnum` (`AIBlueprintHelperLibrary.GetBlackboard` null) "AI_Status" (enumliteral `/Game/My/BP/Enemy/AI_Status` "NewEnumerator0")))))

(fn `UserConstructionScript`)