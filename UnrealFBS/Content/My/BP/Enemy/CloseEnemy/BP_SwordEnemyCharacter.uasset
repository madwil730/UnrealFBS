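; BP_SwordEnemyCharacter is a melee enemy that spawns a BP_Sword and attaches it to its right-hand socket.
; When possessed by an AI controller, it starts a fast looping timer that polls the AI_Status enum in the BP_SwordEnemy controller's blackboard.
; An Attack status plays the downward melee montage, guarded by IsAttack, which a montage-ended handler clears.
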(event `self.ReceiveBeginPlay`
  (bind _returnvalue (`|SpawnActorFromClass` "/Game/My/BP/Enemy/CloseEnemy/BP_Sword.BP_Sword_C" (`KismetMathLibrary.MakeTransform` (0.0 0.0 0.0)) "Undefined" "MultiplyWithRoot" null null))
  (bind _output_get (set `self.weapon` _returnvalue))
  (`SceneComponent.K2_AttachToComponent` (`Actor.RootComponent` _output_get) (`self.Mesh`) "hand_rSocket" "SnapToTarget" "SnapToTarget" "SnapToTarget" true))

(event `self.ReceivePossessed`
  (params (NewController :type "Controller Object Reference"))
  (cast `AIController` NewController)
  (add `AnimInstance.OnMontageEnded` (`SkeletalMeshComponent.GetAnimInstance` (`self.Mesh`)) (`|CreateDelegate` :!event `BP_SwordEnemyCharacter_AutoGenFunc`))
  (`KismetSystemLibrary.K2_SetTimer` null "UpdateAITick" 0.01 true))

(event `self.CapsuleComponent.OnComponentBeginOverlap`
  (params (OverlappedComponent :type "PrimitiveComponent Object Reference") (OtherActor :type "Actor Object Reference") (OtherComp :type "PrimitiveComponent Object Reference") (OtherBodyIndex :type Integer) (bFromSweep :type Boolean) (SweepResult :type "HitResult Structure (by ref)")))

(fn `BP_SwordEnemyCharacter_AutoGenFunc`
  (params (Montage :type "AnimMontage Object Reference") (bInterrupted :type Boolean))
  (set `self.isAttack` false))

(fn `UpdateAITick`
  (bind _asbp_sword_enemy (cast `/Game/My/BP/Enemy/CloseEnemy/BP_SwordEnemy` (`self.GetController`)))
  (bind _output_get (set `self.AIStatus` (cast `/Game/My/BP/Enemy/AI_Status` (`BlackboardComponent.GetValueAsEnum` (`AIBlueprintHelperLibrary.GetBlackboard` _asbp_sword_enemy) "AI_Status"))))
  (switch `/Game/My/BP/Enemy/AI_Status` _output_get
    (:`NewEnumerator2`
      (if (not (`self.isAttack`))
        (set `self.isAttack` true)
        (`self.PlayAnimMontage` "/Game/Characters/Mannequins/Animations/Manny/Standing_Melee_Attack_Downward_Anim_mixamo_com_Montage.Standing_Melee_Attack_Downward_Anim_mixamo_com_Montage")))))

(fn `UserConstructionScript`
  (`parent.UserConstructionScript`))