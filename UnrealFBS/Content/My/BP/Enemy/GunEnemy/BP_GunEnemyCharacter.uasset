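; BP_GunEnemyCharacter is a gun-carrying enemy character that counts as an eliminated target when hit by the player's bullet.
; On BeginPlay it spawns a BP_Weapon and attaches it to the mesh's right-hand rifle socket.
; A capsule overlap with BP_MyBallet increments the player character's TargetsEliminated and runs CheckGoal.
; The enemy then ragdolls with capsule collision disabled, and destroys its gun and itself after a delay.
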(event `self.ReceiveBeginPlay`
  (bind _returnvalue (`|SpawnActorFromClass` "/Game/My/BP/Enemy/GunEnemy/BP_Weapon.BP_Weapon_C" (`KismetMathLibrary.MakeTransform` (0.0 0.0 0.0)) "Undefined" "MultiplyWithRoot" null null))
  (bind _output_get (set `self.Gun` _returnvalue))
  (`SceneComponent.K2_AttachToComponent` (`Actor.RootComponent` _output_get) (`self.Mesh`) "hand_rRifleSocket" "SnapToTarget" "SnapToTarget" "SnapToTarget" true))

(event `self.CapsuleComponent.OnComponentBeginOverlap`
  (params (OverlappedComponent :type "PrimitiveComponent Object Reference") (OtherActor :type "Actor Object Reference") (OtherComp :type "PrimitiveComponent Object Reference") (OtherBodyIndex :type Integer) (bFromSweep :type Boolean) (SweepResult :type "HitResult Structure (by ref)"))
  (cast `/Game/My/BP/BP_MyBallet` OtherActor)
  (bind _asbp_first_person_character (cast `/Game/My/BP/BP_FirstPersonCharacter` (`GameplayStatics.GetPlayerPawn` 0)))
  (set `/Game/My/BP/BP_FirstPersonCharacter.TargetsEliminated` (+ (`/Game/My/BP/BP_FirstPersonCharacter.TargetsEliminated` _asbp_first_person_character) 1) _asbp_first_person_character)
  (`/Game/My/BP/BP_FirstPersonCharacter.CheckGoal` _asbp_first_person_character)
  (`PrimitiveComponent.SetSimulatePhysics` (`self.Mesh`) true)
  (`PrimitiveComponent.SetCollisionEnabled` (`self.CapsuleComponent`) "NoCollision")
  (`KismetSystemLibrary.Delay` 10.0)
  (`self.K2_DestroyActor` (`self.Gun`))
  (`self.K2_DestroyActor`))

(fn `UserConstructionScript`
  (`parent.UserConstructionScript`))