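; BP_EnemyCharacter is a patrolling enemy that loses health when hit by the first-person character.
; Overlapping either patrol point switches the target to the other and writes it to the Blackboard.
; A hit at health one or below spawns an explosion, increments the player's eliminated count, runs its goal check and destroys the enemy.
; The logic setting the initial patrol point is disconnected, leaving BeginPlay empty.
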(event `self.ReceiveBeginPlay`)

(event `self.ReceiveActorBeginOverlap`
  (params (OtherActor :type "Actor Object Reference"))
  (if (== (`self.PatrolPoint1`) OtherActor)
    (set `self.CurrentPatrolPoint` (`self.PatrolPoint2`))
    (`self.UpdatePatrolPointBB` :!label _label)
    (elif (== OtherActor (`self.PatrolPoint2`))
      (set `self.CurrentPatrolPoint` (`self.PatrolPoint1`))
      (goto _label))))

(event `self.ReceiveHit`
  (params (MyComp :type "PrimitiveComponent Object Reference") (Other :type "Actor Object Reference") (OtherComp :type "PrimitiveComponent Object Reference") (bSelfMoved :type Boolean) (HitLocation :type "Vector Structure") (HitNormal :type "Vector Structure") (NormalImpulse :type "Vector Structure") (Hit :type "HitResult Structure (by ref)"))
  (cast `/Game/My/BP/BP_FirstPersonCharacter` Other)
  (if (> (`self.EnemyHealth`) 1)
    (`/Engine/EditorBlueprintResources/StandardMacros.DecrementInt` (`self.EnemyHealth`))
    (else
      (`|SpawnActorFromClass` "/Game/StarterContent/Blueprints/Blueprint_Effect_Explosion.Blueprint_Effect_Explosion_C" (`self.GetTransform`) "Undefined" "MultiplyWithRoot" null null)
      (bind _asbp_first_person_character (cast `/Game/My/BP/BP_FirstPersonCharacter` (`GameplayStatics.GetPlayerCharacter` 0)))
      (`/Engine/EditorBlueprintResources/StandardMacros.IncrementInt` (`/Game/My/BP/BP_FirstPersonCharacter.TargetsEliminated` _asbp_first_person_character)
        (:`  `
          (`/Game/My/BP/BP_FirstPersonCharacter.CheckGoal` _asbp_first_person_character)
          (`self.K2_DestroyActor`))))))

(fn `UserConstructionScript`
  (`parent.UserConstructionScript`))