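; BP_EnemyController is the AI controller for enemies, running BT_EnemyBehavior on begin play.
; Its PawnSensing events feed the blackboard that the behavior tree can act on.
; Seeing a first-person character stores it as the player key.
; Noises within HearingDistance of the controlled pawn record their location and set a heard-sound flag through UpdateSoundBB.
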(event `self.ReceiveBeginPlay`
  (`self.RunBehaviorTree` "/Game/My/BP/Enemy/BT_EnemyBehavior.BT_EnemyBehavior"))

(event `self.PawnSensing.OnSeePawn`
  (params (Pawn :type "Pawn Object Reference"))
  (bind _asbp_first_person_character (cast `/Game/FirstPerson/Blueprints/BP_FirstPersonCharacter` Pawn))
  (`BlackboardComponent.SetValueAsObject` (`AIBlueprintHelperLibrary.GetBlackboard` null) (`self.PlayerKeyName`) _asbp_first_person_character))

(event `self.PawnSensing.OnHearNoise`
  (params (Instigator :type "Pawn Object Reference") (Location :type "Vector Structure (by ref)") (Volume :type "Float (single-precision)"))
  (if (< (`KismetMathLibrary.VSize` (- Location (`self.K2_GetActorLocation` (`self.K2_GetPawn`)))) (`self.HearingDistance`))
    (`self.UpdateSoundBB` Location)))

(fn `UserConstructionScript`)