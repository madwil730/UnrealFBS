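; BP_EnemySpawner is an actor that spawns AI enemies around itself, subject to a cap on enemy count.
; On BeginPlay it sets a timer for SpawnTime, whose event counts all BP_EnemyCharacter actors in the world against MaxEnemies.
; Below the cap, SpawnEnemy spawns a BP_EnemyCharacter running BT_EnemyBehavior at a random navmesh-reachable point within a wide radius of the spawner.
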(event `self.ReceiveBeginPlay`
  (`KismetSystemLibrary.K2_SetTimerDelegate` (delegate `TryTospawnenemy`) (`self.SpawnTime`)))

(event `TryTospawnenemy`
  (bind _outactors (`GameplayStatics.GetAllActorsOfClass` "/Game/My/BP/Enemy/BP_EnemyCharacter.BP_EnemyCharacter_C"))
  (if (< (`KismetArrayLibrary.Array_Length` _outactors) (`self.MaxEnemies`))
    (`self.SpawnEnemy`)))

(fn `UserConstructionScript`)