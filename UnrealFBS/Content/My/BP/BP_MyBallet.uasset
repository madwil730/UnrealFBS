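; BP_MyBallet is a bullet projectile actor that launches itself with a physics impulse along its Arrow component's forward vector on BeginPlay.
; It destroys itself after a fixed delay, or earlier when the Bullet component overlaps any actor other than BP_FirstPersonCharacter.
; The particle trail between two sockets is begun and immediately ended at spawn, and the overlap applies no damage.
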(event `self.ReceiveBeginPlay`
  (bind _particlesystem (`self.ParticleSystem`))
  (`ParticleSystemComponent.BeginTrails` _particlesystem "Trail1" "Trail2" "ETrailWidthMode_FromCentre" 0.0)
  (`ParticleSystemComponent.EndTrails` _particlesystem)
  (`PrimitiveComponent.AddImpulse` (`self.Bullet`) (* (`SceneComponent.GetForwardVector` (`self.Arrow`)) 10000.0) "None" false)
  (`KismetSystemLibrary.Delay` 5.0)
  (`self.K2_DestroyActor`))

(event `self.Bullet.OnComponentBeginOverlap`
  (params (OverlappedComponent :type "PrimitiveComponent Object Reference") (OtherActor :type "Actor Object Reference") (OtherComp :type "PrimitiveComponent Object Reference") (OtherBodyIndex :type Integer) (bFromSweep :type Boolean) (SweepResult :type "HitResult Structure (by ref)"))
  (cast `/Game/My/BP/BP_FirstPersonCharacter` OtherActor
    (:`CastFailed`
      (`self.K2_DestroyActor`))))

(fn `UserConstructionScript`)