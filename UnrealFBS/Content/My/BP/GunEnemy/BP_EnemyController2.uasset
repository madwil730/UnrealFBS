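; AI controller for a gun enemy that runs the BT_EnemyBehavior2 behavior tree on begin play.
; Perception updates write the sensed actor to the Player blackboard key and switch the AI_Status enum depending on whether the stimulus was successfully sensed.
; On lost perception it still stores that actor as Player, changing only the status value, and it does not filter which actors count as targets.
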(event `self.ReceiveBeginPlay`
  (`self.RunBehaviorTree` "/Game/My/BP/GunEnemy/BT_EnemyBehavior2.BT_EnemyBehavior2"))

(event `self.AIPerception.OnTargetPerceptionUpdated`
  (params (Actor :type "Actor Object Reference") (Stimulus :type "AIStimulus Structure"))
  (if (`.bSuccessfullySensed` (break `AIStimulus` Stimulus))
    (`BlackboardComponent.SetValueAsObject` (`AIBlueprintHelperLibrary.GetBlackboard` null) "Player" Actor)
    (`BlackboardComponent.SetValueAsEnum` (`AIBlueprintHelperLibrary.GetBlackboard` null) "AI_Status" (enumliteral `/Game/My/BP/GunEnemy/AI_Status` "NewEnumerator1"))
    (else
      (`BlackboardComponent.SetValueAsObject` (`AIBlueprintHelperLibrary.GetBlackboard` null) "Player" Actor)
      (`BlackboardComponent.SetValueAsEnum` (`AIBlueprintHelperLibrary.GetBlackboard` null) "AI_Status" (enumliteral `/Game/My/BP/GunEnemy/AI_Status` "NewEnumerator0")))))

(fn `UserConstructionScript`)